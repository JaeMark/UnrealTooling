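; BP_GridSimple is an experimental actor that lays out a square grid of mesh instances.
; Its construction script runs two nested loops up to GridSize, adding an instance to an InstancedStaticMesh component at evenly spaced local X and Y offsets.
; The event graph holds only disabled placeholder events, so all of its logic is in the construction script.
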(event EventBeginPlay)

(event Collision|EventActorBeginOverlap
  (params (OtherActor :type Actor%20Object%20Reference)))

(event EventTick
  (params (DeltaSeconds :type Float%20%28single-precision%29)))

(fn ConstructionScript
  (bind _gridsize (Variables|Default|GetGridSize))
  (bind _returnvalue (- _gridsize 1))
  (for _index (range 0 _returnvalue)
    (for _index_2 (range 0 _returnvalue)
      (Components|InstancedStaticMesh|AddInstance (Variables|Default|GetInstancedStaticMesh) (Math|Transform|MakeTransform (Math|Vector|MakeVector (Math|Conversions|ToFloat(Integer) (* _index 160)) (Math|Conversions|ToFloat(Integer) (* _index_2 160)) 0.0)) false))))