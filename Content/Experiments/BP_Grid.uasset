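; BP_Grid is an experimental actor that lays out a square grid of instanced static meshes in its construction script.
; GridSize is capped at 50, and nested loops add one local-space instance per cell on the XY plane.
; Math expressions space cells by mesh bounds plus a gutter, adding an unseeded, asymmetric random offset scaled by MaxRandomOffset.
; The event graph has no active logic.
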(event EventBeginPlay)

(event Collision|EventActorBeginOverlap
  (params (OtherActor :type Actor%20Object%20Reference)))

(event EventTick
  (params (DeltaSeconds :type Float%20%28single-precision%29)))

(fn ConstructionScript
  (bind _instancedstaticmesh (Variables|Default|GetInstancedStaticMesh))
  (bind _maxrandomoffset (Variables|Default|GetMaxRandomOffset))
  (bind (_min _max) (Components|StaticMesh|GetLocalBounds _instancedstaticmesh))
  (bind _returnvalue (/ _maxrandomoffset 2.0))
  (bind _returnvalue_2 (* _maxrandomoffset -1.0))
  (bind _returnvalue_3 (- _max _min))
  (Variables|Default|SetGridSize (Math|Integer|Min(Integer) (Variables|Default|GetGridSize) 50))
  (for _index (range 0 (- (Variables|Default|GetGridSize) 1))
    (for _index_2 (range 0 (- (Variables|Default|GetGridSize) 1))
      (Components|InstancedStaticMesh|AddInstance (Variables|Default|GetInstancedStaticMesh) (Math|Transform|MakeTransform (Math|Vector|MakeVector (|(((N+{6F96A69F-4C1A-7097-588D-ECA1AB09E1CC})*Index)+Offset) (.x _returnvalue_3) (Math|Conversions|ToFloat(Integer) _index) (Math|Random|RandomFloatinRange _returnvalue_2 _returnvalue)) (|(((N+{6F96A69F-4C1A-7097-588D-ECA1AB09E1CC})*Index)+Offset) (.y _returnvalue_3) (Math|Conversions|ToFloat(Integer) _index_2) (Math|Random|RandomFloatinRange _returnvalue_2 _returnvalue)) 0.0)) false))))