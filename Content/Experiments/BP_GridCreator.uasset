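; BP_GridCreator is an experimental actor that builds a square grid of instanced static meshes in its construction script.
; It clamps GridSize to MaxGridSize, then nested loops add one local-space instance per cell to a single InstancedStaticMesh component.
; Math expressions space the cells in X and Y by the mesh's bounds plus a Gutter, so spacing follows the mesh size.
; The event graph holds no active logic.
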(event EventBeginPlay)

(event Collision|EventActorBeginOverlap
  (params (OtherActor :type Actor%20Object%20Reference)))

(event EventTick
  (params (DeltaSeconds :type Float%20%28single-precision%29)))

(fn ConstructionScript
  (bind _instancedstaticmesh (Variables|Default|GetInstancedStaticMesh))
  (bind (_min _max) (Components|StaticMesh|GetLocalBounds _instancedstaticmesh))
  (bind _returnvalue (- _max _min))
  (Variables|Default|SetGridSize (Math|Integer|Min(Integer) (Variables|Default|GetGridSize) (Variables|Default|GetMaxGridSize)))
  (for _index (range 0 (- (Variables|Default|GetGridSize) 1))
    (for _index_2 (range 0 (- (Variables|Default|GetGridSize) 1))
      (Components|InstancedStaticMesh|AddInstance (Variables|Default|GetInstancedStaticMesh) (Math|Transform|MakeTransform (Math|Vector|MakeVector (|((N+{40D4E30C-4267-2068-340A-29871743102E})*Index) (.x _returnvalue) _index) (|((N+{40D4E30C-4267-2068-340A-29871743102E})*Index) (.y _returnvalue) _index_2) 0.0)) false))))